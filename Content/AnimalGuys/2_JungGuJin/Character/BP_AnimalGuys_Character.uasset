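; Networked AnimalGuys player character with movement, MP-limited attack and slide, and hat pickup, using server requests and RepNotify state.
; Attack hits ragdoll the victim, who gets up at a PlayerRevivePoint after a timer.
; In MainGame levels, PlayerState info drives animal mesh and stats, master-posed clothing and spawned hats.
; ChangeCharacterState applies timed scale, speed, jump, ragdoll or freeze effects, then reverts to Normal.
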(event EventBeginPlay
  (Variables|CharacterStat|SetDefaultWalkSpeed (Variables|/Script/Engine.CharacterMovementComponent|GetMaxWalkSpeed (Variables|Character|GetCharacterMovement)))
  (Variables|CharacterStat|SetDefaultJumpVelocity (Variables|/Script/Engine.CharacterMovementComponent|GetJumpZVelocity (Variables|Character|GetCharacterMovement)))
  (Variables|CharacterStat|SetDefaultActorScale3D (Transformation|GetActorScale3D))
  (bind _returnvalue (Game|GetCurrentLevelName true))
  (if (Utilities|String|Contains _returnvalue "MainGame")
    (Character|BindPlayerState)))

(event EventTick
  (params (DeltaSeconds :type Float%20%28single-precision%29))
  (Utilities|FlowControl|Sequence
    (:then_0
      ;[1 1 1] Input Process : UseMP
      (if (and (Variables|Slide|GetCanSlide) (Variables|Slide|GetIsSlide))
        ;;[1 1 1] Decrease Speed While Sliding
        (bind _output_get (Variables|Slide|SetDecressSlideSpeed (- (Variables|Slide|GetDecressSlideSpeed) 3.0)))
        (Variables|/Script/Engine.CharacterMovementComponent|SetMaxWalkSpeed (Variables|Character|GetCharacterMovement) _output_get)
        (bind _asbp_animal_guys_player_state (Utilities|Casting|CastToBP_AnimalGuys_PlayerState (Variables|GetPlayerState)))
        (bind _isnull (Default|UseMPSlide _asbp_animal_guys_player_state (* (Variables|CharacterStat|GetMP_UseSizeOfSlide) (Utilities|Time|GetWorldDeltaSeconds))))
        (if _isnull
          (Variables|Slide|SetCanSlide false)
          (Variables|/Script/Engine.CharacterMovementComponent|SetMaxWalkSpeed (Variables|Character|GetCharacterMovement) (Variables|CharacterStat|GetRunSpeed))
          (Variables|Slide|SetIsSlide false))))
    (:then_1
      (if (not (Variables|Slide|GetIsSlide))
        (bind _asbp_animal_guys_player_state_2 (Utilities|Casting|CastToBP_AnimalGuys_PlayerState (Variables|GetPlayerState)))
        (bind _ismor20 (Default|GetMPSlide _asbp_animal_guys_player_state_2 (* (Variables|CharacterStat|GetGetMPSpeed) (Utilities|Time|GetWorldDeltaSeconds))))
        (if _ismor20
          (Variables|Slide|SetCanSlide true))))
    (:then_2
      ;[1 1 1] 캐릭터 위치값 실시간 보정
      (if (Variables|Default|GetIsRagdoll)
        (Transformation|SetActorLocation (+ (Transformation|GetSocketLocation (Variables|Character|GetMesh) "spine_01") "0, 0,15.000000") false false)))))

(event Input|ActionEvents|InputActionJump
  (params (Key :type Key%20Structure))
  ;[1 1 1] Basic Character Movement
  (:Pressed
    (Character|Jump))
  (:Released
    (Character|StopJumping)))

(event Input|AxisEvents|InputAxisLookUp
  (params (AxisValue :type Float%20%28single-precision%29))
  ;[1 1 1] Basic Character Movement
  (Pawn|Input|AddControllerPitchInput AxisValue))

(event Input|AxisEvents|InputAxisTurn
  (params (AxisValue :type Float%20%28single-precision%29))
  ;[1 1 1] Basic Character Movement
  (Pawn|Input|AddControllerYawInput AxisValue))

(event Input|AxisEvents|InputAxisMoveForward
  (params (AxisValue :type Float%20%28single-precision%29))
  ;[1 1 1] Basic Character Movement
  (Pawn|Input|AddMovementInput (Math|Vector|GetForwardVector (Math|Rotator|MakeRotator 0.0 0.0 (.Yaw (Math|Rotator|BreakRotator (Pawn|GetControlRotation :!class /Script/Engine.Pawn))))) AxisValue false))

(event Input|AxisEvents|InputAxisMoveRight
  (params (AxisValue :type Float%20%28single-precision%29))
  ;[1 1 1] Basic Character Movement
  (Pawn|Input|AddMovementInput (Math|Vector|GetRightVector (Math|Rotator|MakeRotator 0.0 0.0 (.Yaw (Math|Rotator|BreakRotator (Pawn|GetControlRotation :!class /Script/Engine.Pawn))))) AxisValue false))

(event Custom|ReqPickUp
  ;[1 0 0] Run On Server
  (bind _nesresthat (AttachHat|GetNearestHat))
  (Utilities|IsValid _nesresthat
    (:Is%20Valid
      (Utilities|IsValid (Variables|기본/디폴트|GetEquipedHat)
        (:Is%20Valid
          (AttachHat|DisableOwnerHat))
        (:Is%20Not%20Valid
          _))
      (AttachHat|EnableOwnerHat _nesresthat)
      (CallFunction|ResPickup _nesresthat))))

(event Custom|ResPickup
  (params (Hat :type Actor%20Object%20Reference))
  ;[0 0 1] Run On Client
  (Utilities|IsValid Hat
    (:Is%20Valid
      (Utilities|IsValid (Variables|기본/디폴트|GetEquipedHat)
        (:Is%20Valid
          (Class|BPICloth|DetachHat(Message) (Variables|기본/디폴트|GetEquipedHat)))
        (:Is%20Not%20Valid
          _))
      (AttachHat|AttachHat Hat))))

(event Input|ActionEvents|InputActionPickUp
  (params (Key :type Key%20Structure))
  (:Pressed
    (CallFunction|ReqPickUp)))

(event OnComponentHit(CapsuleComponent)
  (params (HitComponent :type Primitive%20Component%20Object%20Reference) (OtherActor :type Actor%20Object%20Reference) (OtherComp :type Primitive%20Component%20Object%20Reference) (NormalImpulse :type Vector :default "0, 0, 0") (Hit :type Hit%20Result%20Structure%20%28by%20ref%29))
  ;[1 0 0] Run On Server : Damage to Other Character
  (if (or (Variables|Attack|GetIsAttacking?) (Variables|Slide|GetSlide))
    (Game|Damage|ApplyDamage OtherActor 1e+01 0 self)))

(event Custom|ResDamage
  (params (DamageCauser :type Actor%20Object%20Reference) (ForceVector :type Vector) (IsAttack :type Boolean))
  ;[0 0.06384 1] Run On Client
  (if IsAttack
    (WhenCrash|DoRagdoll ForceVector)
    (Utilities|Time|SetTimerbyFunctionName 0 "ResRevive" 3.0)
    (else
      (Variables|Attack|SetIsDamaged true))))

(event Custom|ReqAttack
  (params (Attack :type Boolean))
  ;[1 0 0] Run On Server
  (Variables|Attack|SetAttack Attack)
  (if (Variables|Attack|GetCanUseMP)
    (bind _asbp_animal_guys_player_state (Utilities|Casting|CastToBP_AnimalGuys_PlayerState (Variables|GetPlayerState)))
    ;;[1 1 1] Use Stamina
    (if (> (Variables|/Game/AnimalGuys/2_JungGuJin/GameMode/BP_AnimalGuys_PlayerState.BP_AnimalGuys_PlayerState_C|GetCurMP _asbp_animal_guys_player_state) (Math|Conversions|ToFloat(Integer) (Variables|CharacterStat|GetMP_UseSizeOfAttack)))
      (bind _isnull (Default|UseMPAttack _asbp_animal_guys_player_state (Math|Conversions|ToFloat(Integer) (Variables|CharacterStat|GetMP_UseSizeOfAttack))))
      (if _isnull
        (Variables|Attack|SetCanUseMP false)))))

(event Custom|ResRevive
  ;[1 1 1] Do GetUp
  (WhenCrash|DoGetUp)
  ;;[1 1 1] 리스폰 장소 설정
  (bind _returnvalue (Actor|GetActorOfClass "/Game/AnimalGuys/2_JungGuJin/Blueprint/PlayerRevivePoint.PlayerRevivePoint_C"))
  (Utilities|IsValid _returnvalue
    (:Is%20Valid
      (Transformation|SetActorLocationAndRotation (.location (Transformation|GetActorTransform _returnvalue)) (.rotation (Transformation|GetActorTransform _returnvalue))))))

(event Game|Damage|EventAnyDamage
  (params (Damage :type Float%20%28single-precision%29) (DamageType :type Damage%20Type%20Object%20Reference) (InstigatedBy :type Controller%20Object%20Reference) (DamageCauser :type Actor%20Object%20Reference))
  ;[1 0 0] Run On Server : Character Has Damaged
  (bind _asbp_animal_guys_character (Utilities|Casting|CastToBP_AnimalGuys_Character DamageCauser))
  (if (Variables|BP_AnimalGuys_Character_C|GetIsAttack _asbp_animal_guys_character)
    (CallFunction|ResDamage 0 (* (Math|Vector|GetForwardVector (Math|Rotator|FindLookatRotation (Transformation|GetActorLocation _asbp_animal_guys_character) (Transformation|GetActorLocation self))) 2e+04) true)
    (else
      (CallFunction|ResDamage 0 "0, 0, 0" false))))

(event Input|ActionEvents|InputActionAttack
  (params (Key :type Key%20Structure :default "None"))
  (:Pressed
    (if (not (Variables|Default|GetIsJumping?))
      (CallFunction|ReqAttack true))))

(event Custom|ReqSlide
  (params (Slide :type Boolean))
  (Variables|Slide|SetSlide Slide))

(event Input|ActionEvents|InputActionSlide
  (params (Key :type Key%20Structure))
  (:Pressed
    (if (not (Variables|Default|GetIsJumping?))
      (CallFunction|ReqSlide true)))
  (:Released
    (CallFunction|ReqSlide false)))

(event Custom|ChangeCharHatType
  (params (NewCharHatType :type Integer))
  (switch int NewCharHatType
    (:0
      (AttachHat|Haton "Naked"))
    (:1
      (AttachHat|Haton "Preset1"))
    (:2
      (AttachHat|Haton "Preset2"))
    (:3
      (AttachHat|Haton "Preset3"))
    (:4
      (AttachHat|Haton "Preset4"))))

(event Custom|ChangeCharType
  (params (NewCharType :type Integer))
  (switch int NewCharType
    (:0
      (CharShape|ChangeKitty))
    (:1
      (CharShape|ChangePiggy))
    (:2
      (CharShape|ChangeDoggy))
    (:3
      (CharShape|ChangeBunny))))

(event Custom|ChangeCharClothType
  (params (NewCharClothType :type Integer))
  (switch int NewCharClothType
    (:0
      (ClothColor|ClothTypeNaked))
    (:1
      (ClothColor|ClothTypeA))
    (:2
      (ClothColor|ClothTypeB))
    (:3
      (ClothColor|ClothTypeC))))

(fn ConstructionScript)

(fn OnRepSlide
  (PlayMotion|SetSlide (Variables|Slide|GetSlide)))

(fn SetSlide
  (params (Slide :type Boolean))
  (bind _defaultslidespeed (Variables|CharacterStat|GetDefaultSlideSpeed))
  (if Slide
    (if (Variables|Slide|GetCanSlide)
      (Variables|Slide|SetIsSlide true)
      (Variables|/Script/Engine.CharacterMovementComponent|SetMaxWalkSpeed (Variables|Character|GetCharacterMovement) _defaultslidespeed)
      (Variables|Slide|SetDecressSlideSpeed _defaultslidespeed))
    (else
      (Variables|Slide|SetIsSlide false)
      (Variables|/Script/Engine.CharacterMovementComponent|SetMaxWalkSpeed (Variables|Character|GetCharacterMovement) (Variables|CharacterStat|GetRunSpeed)))))

(fn OnRepAttack
  (PlayMotion|SetAttack (Variables|Attack|GetAttack)))

(fn SetAttack
  (params (Attack :type Boolean))
  (if Attack
    (bind _asbp_animal_guys_player_state (Utilities|Casting|CastToBP_AnimalGuys_PlayerState (Variables|GetPlayerState)))
    (if (> (Variables|/Game/AnimalGuys/2_JungGuJin/GameMode/BP_AnimalGuys_PlayerState.BP_AnimalGuys_PlayerState_C|GetCurMP _asbp_animal_guys_player_state) (Math|Conversions|ToFloat(Integer) (Variables|CharacterStat|GetMP_UseSizeOfAttack)))
      (Variables|Attack|SetIsAttack true))))

(fn ChangeKitty
  (Rendering|SetVisibility (Variables|Default|GetSkeletalMesh) false false)
  (Class|SkeletalMeshComponent|SetAnimClass (Variables|Character|GetMesh) "/Game/AnimalGuys/2_JungGuJin/Character/0_Kitty/Animation/ABP_AnimalKitty.ABP_AnimalKitty_C")
  (Class|SkinnedMeshComponent|SetSkeletalMesh (Variables|Character|GetMesh) "/Game/Cute_Little_Animals/Kitty/Mesh/SK_Kitty.SK_Kitty" true)
  (Character|CharacterStat 30 30 40 8e+02 6e+02 6e+02 1e+02 3.0 2.0)
  (Variables|Default|SetAnimalType 0))

(fn CharacterStat
  (params (GetMPSpeed :type Integer) (MP_UseSizeOfSlide :type Integer) (MP_UseSizeOfAttack :type Integer) (SlideSpeed :type Float%20%28single-precision%29) (RunSpeed :type Float%20%28single-precision%29) (Jump%20Z%20Velocity :type Float%20%28single-precision%29) (MaxMP :type Float%20%28single-precision%29) (AttackCoolTime :type Float%20%28single-precision%29) (DownTimeLength :type Float%20%28single-precision%29))
  (Variables|CharacterStat|SetMP_UseSizeOfSlide MP_UseSizeOfSlide)
  (Variables|CharacterStat|SetDefaultSlideSpeed SlideSpeed)
  (bind _output_get (Variables|CharacterStat|SetRunSpeed RunSpeed))
  (Variables|/Script/Engine.CharacterMovementComponent|SetMaxWalkSpeed (Variables|Character|GetCharacterMovement) _output_get)
  (Variables|/Script/Engine.CharacterMovementComponent|SetJumpZVelocity (Variables|Character|GetCharacterMovement) Jump%20Z%20Velocity)
  (bind _asbp_animal_guys_player_state (Utilities|Casting|CastToBP_AnimalGuys_PlayerState (Variables|GetPlayerState)))
  (Variables|/Game/AnimalGuys/2_JungGuJin/GameMode/BP_AnimalGuys_PlayerState.BP_AnimalGuys_PlayerState_C|SetMaxMP _asbp_animal_guys_player_state MaxMP)
  (Variables|CharacterStat|SetAttackCoolTime AttackCoolTime)
  (Variables|CharacterStat|SetMP_UseSizeOfAttack MP_UseSizeOfAttack)
  (Variables|CharacterStat|SetGetMPSpeed GetMPSpeed)
  (Variables|CharacterStat|SetDownTimeLength DownTimeLength))

(fn GetNearestHat
  (for _array_element (Collision|GetOverlappingActors (Variables|Collision|GetCapsuleComponent) "/Game/AnimalGuys/2_JungGuJin/Cloth/Hat/HatParent/BP_Hat.BP_Hat_C" :!class /Script/Engine.PrimitiveComponent)
    (if (Utilities|DoesObjectImplementInterface _array_element "/Game/AnimalGuys/2_JungGuJin/Cloth/Hat/BPI_Cloth.BPI_Cloth_C")
      (if (> (LocalVariables|GetNearestDist) (Math|Vector|Distance(Vector) (Transformation|GetActorLocation) (Transformation|GetActorLocation _array_element)))
        (LocalVariables|SetNearestDist (Math|Vector|Distance(Vector) (Transformation|GetActorLocation) (Transformation|GetActorLocation _array_element)))
        (LocalVariables|SetNearestActor _array_element))))
  (return (LocalVariables|GetNearestActor)))

(fn DisableOwnerHat
  (bind _equipedhat (Variables|기본/디폴트|GetEquipedHat))
  (Utilities|IsValid _equipedhat
    (:Is%20Valid
      (Actor|SetOwner _equipedhat 0))))

(fn EnableOwnerHat
  (params (EquipHat :type Actor%20Object%20Reference))
  (Actor|SetOwner (Pawn|GetController)))

(fn AttachHat
  (params (EquipedHat :type Actor%20Object%20Reference))
  (bind _output_get (Variables|기본/디폴트|SetEquipedHat EquipedHat))
  (Class|BPICloth|AttachHat(Message) _output_get self))

(fn ChangePiggy
  (Rendering|SetVisibility (Variables|Default|GetSkeletalMesh) false false)
  (Class|SkeletalMeshComponent|SetAnimClass (Variables|Character|GetMesh) "/Game/AnimalGuys/2_JungGuJin/Character/1_Piggy/Animation/ABP_AnimalPiggy.ABP_AnimalPiggy_C")
  (Class|SkinnedMeshComponent|SetSkeletalMesh (Variables|Character|GetMesh) "/Game/Cute_Little_Animals/Piggy/Mesh/SK_Piggy.SK_Piggy" true)
  (Character|CharacterStat 30 30 40 8e+02 6e+02 6e+02 1e+02 3.0 2.0)
  (Variables|Default|SetAnimalType 1))

(fn ChangeDoggy
  (Development|PrintString "Hello" true true "(R=1.000000,G=0.000000,B=0.760268,A=1.000000)" 3e+01)
  (Rendering|SetVisibility (Variables|Default|GetSkeletalMesh) false false)
  (Class|SkeletalMeshComponent|SetAnimClass (Variables|Character|GetMesh) "/Game/AnimalGuys/2_JungGuJin/Character/2_Doggy/Animation/ABP_AnimDoggy.ABP_AnimDoggy_C")
  (Class|SkinnedMeshComponent|SetSkeletalMesh (Variables|Character|GetMesh) "/Game/Cute_Little_Animals/Doggy/Mesh/SK_Doggy.SK_Doggy" true)
  (Character|CharacterStat 30 30 40 8e+02 6e+02 6e+02 1e+02 3.0 2.0)
  (Variables|Default|SetAnimalType 2))

(fn ChangeBunny
  (Rendering|SetVisibility (Variables|Default|GetSkeletalMesh) false false)
  (Class|SkeletalMeshComponent|SetAnimClass (Variables|Character|GetMesh) "/Game/AnimalGuys/2_JungGuJin/Character/3_Bunny/Animation/ABP_AnimBunny.ABP_AnimBunny_C")
  (Class|SkinnedMeshComponent|SetSkeletalMesh (Variables|Character|GetMesh) "/Game/Cute_Little_Animals/Bunny/Mesh/SK_Bunny.SK_Bunny" true)
  (Character|CharacterStat 30 30 40 8e+02 6e+02 6e+02 1e+02 3.0 2.0)
  (Variables|Default|SetAnimalType 3))

(fn ClothTypeA
  (bind _skeletalmesh (Variables|Default|GetSkeletalMesh))
  (bind _skeletalmesh_2 (Variables|Default|GetSkeletalMesh))
  (bind _skeletalmesh_3 (Variables|Default|GetSkeletalMesh))
  (bind _skeletalmesh_4 (Variables|Default|GetSkeletalMesh))
  (bind _skeletalmesh_5 (Variables|Default|GetSkeletalMesh))
  (Rendering|SetVisibility _skeletalmesh_3 true false)
  (Utilities|Casting|CastToBP_AnimalGuys_PlayerState (Variables|GetPlayerState))
  (switch int (Variables|Default|GetAnimalType)
    (:0
      (Rendering|Material|SetMaterial _skeletalmesh_3 0 "/Game/AnimalGuys/2_JungGuJin/Character/0_Kitty/Material/MI_Kitty_A.MI_Kitty_A")
      (Class|SkeletalMeshComponent|SetAnimClass _skeletalmesh_4 "/Game/AnimalGuys/2_JungGuJin/Character/0_Kitty/Animation/ABP_AnimalKitty.ABP_AnimalKitty_C")
      (Class|SkinnedMeshComponent|SetSkeletalMesh _skeletalmesh_4 "/Game/AnimalGuys/2_JungGuJin/Character/0_Kitty/Mesh/SK_Kitty_MyClothes.SK_Kitty_MyClothes" true)
      (Class|SkinnedMeshComponent|SetMasterPoseComponent _skeletalmesh_4 (Variables|Character|GetMesh) false))
    (:1
      (Rendering|Material|SetMaterial _skeletalmesh_3 0 "/Game/AnimalGuys/2_JungGuJin/Character/1_Piggy/Material/MI_Piggy_A.MI_Piggy_A")
      (Class|SkeletalMeshComponent|SetAnimClass _skeletalmesh "/Game/AnimalGuys/2_JungGuJin/Character/1_Piggy/Animation/ABP_AnimalPiggy.ABP_AnimalPiggy_C")
      (Class|SkinnedMeshComponent|SetSkeletalMesh _skeletalmesh "/Game/Cute_Little_Animals/Piggy/Mesh/SK_Piggy_Clothes.SK_Piggy_Clothes" true)
      (Class|SkinnedMeshComponent|SetMasterPoseComponent _skeletalmesh (Variables|Character|GetMesh) false))
    (:2
      (Rendering|Material|SetMaterial _skeletalmesh_3 0 "/Game/AnimalGuys/2_JungGuJin/Character/2_Doggy/Material/MI_Doggy_A.MI_Doggy_A")
      (Class|SkeletalMeshComponent|SetAnimClass _skeletalmesh_2 "/Game/AnimalGuys/2_JungGuJin/Character/2_Doggy/Animation/ABP_AnimDoggy.ABP_AnimDoggy_C")
      (Class|SkinnedMeshComponent|SetSkeletalMesh _skeletalmesh_2 "/Game/Cute_Little_Animals/Doggy/Mesh/SK_Doggy_clothes.SK_Doggy_clothes" true)
      (Class|SkinnedMeshComponent|SetMasterPoseComponent _skeletalmesh_2 (Variables|Character|GetMesh) false))
    (:3
      (Rendering|Material|SetMaterial _skeletalmesh_3 0 "/Game/AnimalGuys/2_JungGuJin/Character/3_Bunny/Material/MI_Bunny_A.MI_Bunny_A")
      (Class|SkeletalMeshComponent|SetAnimClass _skeletalmesh_5 "/Game/AnimalGuys/2_JungGuJin/Character/3_Bunny/Animation/ABP_AnimBunny.ABP_AnimBunny_C")
      (Class|SkinnedMeshComponent|SetSkeletalMesh _skeletalmesh_5 "/Game/Cute_Little_Animals/Bunny/Mesh/SK_Bunny_Clothes.SK_Bunny_Clothes" true)
      (Class|SkinnedMeshComponent|SetMasterPoseComponent _skeletalmesh_5 (Variables|Character|GetMesh) false))))

(fn ClothTypeNaked
  (Utilities|Casting|CastToBP_AnimalGuys_PlayerState (Variables|GetPlayerState))
  (switch int (Variables|Default|GetAnimalType)
    (:0
      _)
    (:1
      _)
    (:2
      _)
    (:3
      _))
  (Rendering|SetVisibility (Variables|Default|GetSkeletalMesh) false false))

(fn ClothTypeB
  (bind _skeletalmesh (Variables|Default|GetSkeletalMesh))
  (bind _skeletalmesh_2 (Variables|Default|GetSkeletalMesh))
  (bind _skeletalmesh_3 (Variables|Default|GetSkeletalMesh))
  (bind _skeletalmesh_4 (Variables|Default|GetSkeletalMesh))
  (bind _skeletalmesh_5 (Variables|Default|GetSkeletalMesh))
  (Rendering|SetVisibility _skeletalmesh_3 true false)
  (Utilities|Casting|CastToBP_AnimalGuys_PlayerState (Variables|GetPlayerState))
  (switch int (Variables|Default|GetAnimalType)
    (:0
      (Rendering|Material|SetMaterial _skeletalmesh_3 0 "/Game/AnimalGuys/2_JungGuJin/Character/0_Kitty/Material/MI_Kitty_B.MI_Kitty_B")
      (Class|SkeletalMeshComponent|SetAnimClass _skeletalmesh_4 "/Game/AnimalGuys/2_JungGuJin/Character/0_Kitty/Animation/ABP_AnimalKitty.ABP_AnimalKitty_C")
      (Class|SkinnedMeshComponent|SetSkeletalMesh _skeletalmesh_4 "/Game/AnimalGuys/2_JungGuJin/Character/0_Kitty/Mesh/SK_Kitty_MyClothes.SK_Kitty_MyClothes" true)
      (Class|SkinnedMeshComponent|SetMasterPoseComponent _skeletalmesh_4 (Variables|Character|GetMesh) false))
    (:1
      (Rendering|Material|SetMaterial _skeletalmesh_3 0 "/Game/AnimalGuys/2_JungGuJin/Character/1_Piggy/Material/MI_Piggy_B.MI_Piggy_B")
      (Class|SkeletalMeshComponent|SetAnimClass _skeletalmesh "/Game/AnimalGuys/2_JungGuJin/Character/1_Piggy/Animation/ABP_AnimalPiggy.ABP_AnimalPiggy_C")
      (Class|SkinnedMeshComponent|SetSkeletalMesh _skeletalmesh "/Game/Cute_Little_Animals/Piggy/Mesh/SK_Piggy_Clothes.SK_Piggy_Clothes" true)
      (Class|SkinnedMeshComponent|SetMasterPoseComponent _skeletalmesh (Variables|Character|GetMesh) false))
    (:2
      (Rendering|Material|SetMaterial _skeletalmesh_3 0 "/Game/AnimalGuys/2_JungGuJin/Character/2_Doggy/Material/MI_Doggy_B.MI_Doggy_B")
      (Class|SkeletalMeshComponent|SetAnimClass _skeletalmesh_2 "/Game/AnimalGuys/2_JungGuJin/Character/2_Doggy/Animation/ABP_AnimDoggy.ABP_AnimDoggy_C")
      (Class|SkinnedMeshComponent|SetSkeletalMesh _skeletalmesh_2 "/Game/Cute_Little_Animals/Doggy/Mesh/SK_Doggy_clothes.SK_Doggy_clothes" true)
      (Class|SkinnedMeshComponent|SetMasterPoseComponent _skeletalmesh_2 (Variables|Character|GetMesh) false))
    (:3
      (Rendering|Material|SetMaterial _skeletalmesh_3 0 "/Game/AnimalGuys/2_JungGuJin/Character/3_Bunny/Material/MI_Bunny_B.MI_Bunny_B")
      (Class|SkeletalMeshComponent|SetAnimClass _skeletalmesh_5 "/Game/AnimalGuys/2_JungGuJin/Character/3_Bunny/Animation/ABP_AnimBunny.ABP_AnimBunny_C")
      (Class|SkinnedMeshComponent|SetSkeletalMesh _skeletalmesh_5 "/Game/Cute_Little_Animals/Bunny/Mesh/SK_Bunny_Clothes.SK_Bunny_Clothes" true)
      (Class|SkinnedMeshComponent|SetMasterPoseComponent _skeletalmesh_5 (Variables|Character|GetMesh) false))))

(fn ClothTypeC
  (bind _skeletalmesh (Variables|Default|GetSkeletalMesh))
  (bind _skeletalmesh_2 (Variables|Default|GetSkeletalMesh))
  (bind _skeletalmesh_3 (Variables|Default|GetSkeletalMesh))
  (bind _skeletalmesh_4 (Variables|Default|GetSkeletalMesh))
  (bind _skeletalmesh_5 (Variables|Default|GetSkeletalMesh))
  (Rendering|SetVisibility _skeletalmesh_3 true false)
  (Utilities|Casting|CastToBP_AnimalGuys_PlayerState (Variables|GetPlayerState))
  (switch int (Variables|Default|GetAnimalType)
    (:0
      (Rendering|Material|SetMaterial _skeletalmesh_3 0 "/Game/AnimalGuys/2_JungGuJin/Character/0_Kitty/Material/MI_Kitty_C.MI_Kitty_C")
      (Class|SkeletalMeshComponent|SetAnimClass _skeletalmesh_4 "/Game/AnimalGuys/2_JungGuJin/Character/0_Kitty/Animation/ABP_AnimalKitty.ABP_AnimalKitty_C")
      (Class|SkinnedMeshComponent|SetSkeletalMesh _skeletalmesh_4 "/Game/AnimalGuys/2_JungGuJin/Character/0_Kitty/Mesh/SK_Kitty_MyClothes.SK_Kitty_MyClothes" true)
      (Class|SkinnedMeshComponent|SetMasterPoseComponent _skeletalmesh_4 (Variables|Character|GetMesh) false))
    (:1
      (Rendering|Material|SetMaterial _skeletalmesh_3 0 "/Game/AnimalGuys/2_JungGuJin/Character/1_Piggy/Material/MI_Piggy_C.MI_Piggy_C")
      (Class|SkeletalMeshComponent|SetAnimClass _skeletalmesh "/Game/AnimalGuys/2_JungGuJin/Character/1_Piggy/Animation/ABP_AnimalPiggy.ABP_AnimalPiggy_C")
      (Class|SkinnedMeshComponent|SetSkeletalMesh _skeletalmesh "/Game/Cute_Little_Animals/Piggy/Mesh/SK_Piggy_Clothes.SK_Piggy_Clothes" true)
      (Class|SkinnedMeshComponent|SetMasterPoseComponent _skeletalmesh (Variables|Character|GetMesh) false))
    (:2
      (Rendering|Material|SetMaterial _skeletalmesh_3 0 "/Game/AnimalGuys/2_JungGuJin/Character/2_Doggy/Material/MI_Doggy_C.MI_Doggy_C")
      (Class|SkeletalMeshComponent|SetAnimClass _skeletalmesh_2 "/Game/AnimalGuys/2_JungGuJin/Character/2_Doggy/Animation/ABP_AnimDoggy.ABP_AnimDoggy_C")
      (Class|SkinnedMeshComponent|SetSkeletalMesh _skeletalmesh_2 "/Game/Cute_Little_Animals/Doggy/Mesh/SK_Doggy_clothes.SK_Doggy_clothes" true)
      (Class|SkinnedMeshComponent|SetMasterPoseComponent _skeletalmesh_2 (Variables|Character|GetMesh) false))
    (:3
      (Rendering|Material|SetMaterial _skeletalmesh_3 0 "/Game/AnimalGuys/2_JungGuJin/Character/3_Bunny/Material/MI_Bunny_C.MI_Bunny_C")
      (Class|SkeletalMeshComponent|SetAnimClass _skeletalmesh_5 "/Game/AnimalGuys/2_JungGuJin/Character/3_Bunny/Animation/ABP_AnimBunny.ABP_AnimBunny_C")
      (Class|SkinnedMeshComponent|SetSkeletalMesh _skeletalmesh_5 "/Game/Cute_Little_Animals/Bunny/Mesh/SK_Bunny_Clothes.SK_Bunny_Clothes" true)
      (Class|SkinnedMeshComponent|SetMasterPoseComponent _skeletalmesh_5 (Variables|Character|GetMesh) false))))

(fn DoRagdoll
  (params (ForceVector :type Vector))
  (if (not (Variables|Default|GetIsRagdoll))
    (Variables|Default|SetIsRagdoll true)
    (Physics|SetSimulatePhysics (Variables|Character|GetMesh) true)
    (Physics|AddImpulse (Variables|Character|GetMesh) ForceVector "None" false)
    (Pawn|Components|CharacterMovement|SetMovementMode (Variables|Character|GetCharacterMovement) "MOVE_None" 0)))

(fn DoGetUp
  (Variables|Default|SetIsRagdoll false)
  (Physics|SetSimulatePhysics (Variables|Character|GetMesh) false)
  (Transformation|AttachComponentToComponent (Variables|Character|GetMesh) (Variables|Collision|GetCapsuleComponent) "None" "KeepRelative" "KeepRelative" "KeepRelative" true)
  (Transformation|SetRelativeLocationAndRotation (Variables|Character|GetMesh) "0, 0,-49.000000" "0,-90.000000, 0" false false)
  (Pawn|Components|CharacterMovement|SetMovementMode (Variables|Character|GetCharacterMovement) "MOVE_Walking" 0))

(fn Haton
  (params (HatName :type String))
  (bind _returnvalue (Math|Transform|MakeTransform "-999.000000,-999.000000,-999.000000"))
  (Utilities|IsValid (Variables|기본/디폴트|GetEquipedHat)
    (:Is%20Valid
      (Class|BPICloth|DetachHat(Message) (Variables|기본/디폴트|GetEquipedHat))
      (Actor|DestroyActor (Variables|기본/디폴트|GetEquipedHat))
      (Variables|기본/디폴트|SetEquipedHat 0))
    (:Is%20Not%20Valid
      _))
  (switch string HatName
    (:Preset1
      (bind _returnvalue_2 (Game|SpawnActorfromClass "/Game/AnimalGuys/2_JungGuJin/Cloth/Hat/Bariation/BariationBigGreen.BariationBigGreen_C" _returnvalue "Undefined" 0 0))
      (bind _output_get (Variables|기본/디폴트|SetEquipedHat _returnvalue_2))
      (Class|BPICloth|AttachHat(Message) _output_get self))
    (:Preset2
      (bind _returnvalue_3 (Game|SpawnActorfromClass "/Game/AnimalGuys/2_JungGuJin/Cloth/Hat/Bariation/BariationBigRed.BariationBigRed_C" _returnvalue "Undefined" 0 0))
      (bind _output_get_2 (Variables|기본/디폴트|SetEquipedHat _returnvalue_3))
      (Class|BPICloth|AttachHat(Message) _output_get_2 self))
    (:Preset3
      (bind _returnvalue_4 (Game|SpawnActorfromClass "/Game/AnimalGuys/2_JungGuJin/Cloth/Hat/Bariation/BariationSmallGreen.BariationSmallGreen_C" _returnvalue "Undefined" 0 0))
      (bind _output_get_3 (Variables|기본/디폴트|SetEquipedHat _returnvalue_4))
      (Class|BPICloth|AttachHat(Message) _output_get_3 self))
    (:Preset4
      (bind _returnvalue_5 (Game|SpawnActorfromClass "/Game/AnimalGuys/2_JungGuJin/Cloth/Hat/Bariation/BariationSmallGreenBox.BariationSmallGreenBox_C" _returnvalue "Undefined" 0 0))
      (bind _output_get_4 (Variables|기본/디폴트|SetEquipedHat _returnvalue_5))
      (Class|BPICloth|AttachHat(Message) _output_get_4 self))))

(fn SetCharacterRandomLocation
  (Transformation|SetActorLocation (Math|Random|RandomPointinBoundingBox (Transformation|GetActorLocation) "300.000000,300.000000, 0") false false))

(fn ChangePlayerInfo
  (params (PlayerInfo :type ST%20Player%20Info%20Structure))
  (bind (_playerid _playerpwd _playername _playergold _playerexp _playerlevel _playerchartype _playercharbodyslot _playercharheadslot) (Utilities|Struct|BreakST_PlayerInfo PlayerInfo))
  (CallFunction|ChangeCharType _playerchartype)
  (CallFunction|ChangeCharHatType _playercharbodyslot)
  (CallFunction|ChangeCharClothType _playercharheadslot))

(fn BindPlayerState
  (bind _asbp_animal_guys_player_state (Utilities|Casting|CastToBP_AnimalGuys_PlayerState (Variables|GetPlayerState))
    (:then
      (EventDispatchers|BindEventtoEventDispatcherChangePlayerInfo _asbp_animal_guys_player_state (EventDispatchers|CreateEvent :!event ChangePlayerInfo))
      (Character|ChangePlayerInfo (Variables|/Game/AnimalGuys/2_JungGuJin/GameMode/BP_AnimalGuys_PlayerState.BP_AnimalGuys_PlayerState_C|GetST_PlayerInfo _asbp_animal_guys_player_state)))
    (:CastFailed
      (Utilities|Time|SetTimerbyFunctionName 0 "BindPlayerState" 0.1))))

(fn ChangeCharacterState
  (params (CharacterState :type EN_CharacterState%20Enum :default "NewEnumerator0"))
  (bind _output_get (Variables|ItemGain|SetCharacterState CharacterState))
  (Default|CallEventDispatcherChangeCharacterState _output_get)
  (switch Utilities|FlowControl|Switch|SwitchonEN_CharacterState _output_get
    (:NewEnumerator9
      (Pawn|Components|CharacterMovement|SetMovementMode (Variables|Character|GetCharacterMovement) "MOVE_Walking" 0)
      (Transformation|SetActorScale3D self (Variables|CharacterStat|GetDefaultActorScale3D))
      (Variables|/Script/Engine.CharacterMovementComponent|SetMaxWalkSpeed (Variables|Character|GetCharacterMovement) (Variables|CharacterStat|GetDefaultWalkSpeed))
      (Variables|/Script/Engine.CharacterMovementComponent|SetJumpZVelocity (Variables|Character|GetCharacterMovement) (Variables|CharacterStat|GetDefaultJumpVelocity))
      (if (Variables|Default|GetIsRagdoll)
        (WhenCrash|DoGetUp))
      (Utilities|Time|ClearTimerbyFunctionName 0 "FinishCharacterStatus"))
    (:NewEnumerator0
      (Transformation|SetActorScale3D self (* (Variables|CharacterStat|GetDefaultActorScale3D) 2.0))
      (Utilities|Time|ClearTimerbyFunctionName 0 "FinishCharacterStatus" :!label _label)
      (Utilities|Time|SetTimerbyFunctionName 0 "FinishCharacterStatus" (Variables|ItemGain|GetItemAffectTime)))
    (:NewEnumerator1
      (Transformation|SetActorScale3D self (* (Variables|CharacterStat|GetDefaultActorScale3D) 0.5))
      (goto _label))
    (:NewEnumerator2
      (Variables|/Script/Engine.CharacterMovementComponent|SetMaxWalkSpeed (Variables|Character|GetCharacterMovement) (* (Variables|CharacterStat|GetDefaultWalkSpeed) 4.0))
      (goto _label))
    (:NewEnumerator3
      (Variables|/Script/Engine.CharacterMovementComponent|SetMaxWalkSpeed (Variables|Character|GetCharacterMovement) (* (Variables|CharacterStat|GetDefaultWalkSpeed) 0.25))
      (goto _label))
    (:NewEnumerator4
      (bind _output_get_2 (Variables|/Script/Engine.CharacterMovementComponent|SetJumpZVelocity (Variables|Character|GetCharacterMovement) (* (Variables|CharacterStat|GetDefaultJumpVelocity) 4.0)))
      (Development|PrintString (Utilities|String|ToString(Float) _output_get_2))
      (goto _label))
    (:NewEnumerator5
      (bind _output_get_3 (Variables|/Script/Engine.CharacterMovementComponent|SetJumpZVelocity (Variables|Character|GetCharacterMovement) (* (Variables|CharacterStat|GetDefaultJumpVelocity) 0.25)))
      (Development|PrintString (Utilities|String|ToString(Float) _output_get_3))
      (goto _label))
    (:NewEnumerator6
      (WhenCrash|DoRagdoll "0, 0, 0")
      (goto _label))
    (:NewEnumerator7
      (Pawn|Components|CharacterMovement|SetMovementMode (Variables|Character|GetCharacterMovement) "MOVE_None" 0)
      (goto _label))))

(fn FinishCharacterStatus
  (CallFunction|ChangeCharacterState "NewEnumerator9"))